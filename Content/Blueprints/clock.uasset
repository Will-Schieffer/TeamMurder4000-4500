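; Interactive clock puzzle Blueprint with a close-up view and a clickable control that turns its hand.
; ClockInteractedWIth flip-flops between blending the view to the clock with a mouse cursor and input ignored, and restoring the default camera, controls and notifying BP_Player.
; Each click on Cube1 plays a sound and steps the Arrow, calling that same toggle when its world roll exactly equals the target angle.
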(event OnClicked(Cube1)
  (params (TouchedComponent :type Primitive%20Component%20Object%20Reference) (ButtonPressed :type Key%20Structure :default "None"))
  (Audio|PlaySound2D "/Game/SoundFX/MouseClick.MouseClick" 1.0 1.0 0.0 0 0)
  (Transformation|AddLocalRotation (Variables|Default|GetArrow) "0.000000,0.000000,-30.000000" false false)
  (if (== (.roll (Transformation|GetWorldRotation (Variables|Default|GetArrow))) -9e+01)
    (CallFunction|ClockInteractedWIth)))

(event Custom|ClockInteractedWIth
  (bind _returnvalue (Game|GetPlayerController 0))
  (bind _returnvalue_2 (Game|GetPlayerController 0))
  (Utilities|FlowControl|FlipFlop
    (:A
      (Game|Player|SetViewTargetwithBlend _returnvalue_2 self 0.5 "VTBlend_Linear" 0.0 false)
      (Input|SetIgnoreLookInput _returnvalue_2 true)
      (Input|SetIgnoreMoveInput _returnvalue_2 true)
      (Variables|/Script/Engine.PlayerController|SetbShowMouseCursor (Game|GetPlayerController 0) true))
    (:B
      (Default|ResetCam (Variables|Default|GetDefault%20Cam))
      (Input|SetIgnoreLookInput _returnvalue false)
      (Input|SetIgnoreMoveInput _returnvalue false)
      (Variables|/Script/Engine.PlayerController|SetbShowMouseCursor (Game|GetPlayerController 0) false)
      (bind _asbp_player (Utilities|Casting|CastToBP_Player (Game|GetPlayerCharacter 0)))
      (Default|EndClockInteractions _asbp_player))))

(event EventBeginPlay)

(fn ConstructionScript)
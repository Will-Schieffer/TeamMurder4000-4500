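; BP_PuzzleGate tracks the dumbwaiter puzzle's six slot flags and a count of collected souvenirs.
; CheckDumbwaiter plays a click, waits briefly, then either plays an error sound or, if all slots are true, runs success sounds once and calls CompletedPuzzle.
; CompletedPuzzle removes the unsolved background widget and tells BP_Player the dumbwaiter is solved.
; CollectItem only increments the souvenir counter, which the puzzle check does not read.
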(event Custom|Collect%20Item
  (Math|Integer|IncrementInt (Variables|Default|GetsouvenirsCollected)))

(event Custom|Check%20Dumbwaiter
  (params (UI :type WB%20Background%20Object%20Reference))
  (Audio|PlaySound2D "/Game/SoundFX/MouseClick.MouseClick" 1.0 1.0 0.0 0 0)
  (Utilities|FlowControl|Delay 0.4)
  (if (Math|Boolean|ANDBoolean (== (Variables|Default|GetSlot1) true) (== (Variables|Default|GetSlot2) true) (== (Variables|Default|GetSlot3) true) (== (Variables|Default|GetSlot4) true) (== (Variables|Default|GetSlot5) true) (== (Variables|Default|GetSlot6) true))
    (Utilities|FlowControl|DoOnce false
      (:Completed
        (Audio|PlaySound2D "/Game/SoundFX/NotifyEffect.NotifyEffect" 1.0 1.0 0.0 0 0)
        (Utilities|FlowControl|Delay 0.5)
        (Audio|PlaySound2D "/Game/SoundFX/Pulley.Pulley" 1.0 1.0 0.0 0 0)
        (CallFunction|CompletedPuzzle)))
    (else
      (Audio|PlaySound2D "/Game/SoundFX/Error_wav.Error_wav" 1.0 1.0 0.0 0 0))))

(event Custom|Completed%20Puzzle
  (Development|PrintString "complete!!")
  (Widget|RemovefromParent (Variables|Default|GetUnsolvedBG))
  (Development|PrintString "Tried to remove from BG")
  (bind _asbp_player (Utilities|Casting|CastToBP_Player (Game|GetPlayerCharacter 0)))
  (Default|DumbWaiterSolved _asbp_player))

(fn ConstructionScript)
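; Fixed cinematic camera that takes over the player's view when the player pawn enters its box, or shortly after BeginPlay if flagged as starting camera.
; Overlap plays a wing-flap sound and runs a timeline fade through a post-process blendable material, switching view and enabling tick at full alpha.
; Tick smoothly aims at the player within clamped pitch and yaw.
; ActivateTint animates the camera's post-process weight, guarded against retriggering.
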(event OnComponentBeginOverlap(Box)
  (params (OverlappedComponent :type Primitive%20Component%20Object%20Reference) (OtherActor :type Actor%20Object%20Reference) (OtherComp :type Primitive%20Component%20Object%20Reference) (OtherBodyIndex :type Integer) (bFromSweep :type Boolean) (SweepResult :type Hit%20Result%20Structure%20%28by%20ref%29))
  (if (== OtherActor (Game|Player|GetPlayerPawn 0))
    (bind _returnvalue (Rendering|Material|CreateDynamicMaterialInstance "/Game/Materials/M_Fade.M_Fade" "None" "None" :!class /Script/Engine.KismetMaterialLibrary))
    (Variables|Default|SetFadeMaterial _returnvalue)
    (Audio|PlaySound2D "/Game/SoundFX/WingsFlapping3.WingsFlapping3" 1.0 1.0 0.0 0 0)
    (bind _returnvalue_2 (Actor|GetActorOfClass "/Script/Engine.PostProcessVolume"))
    (Rendering|AddorUpdateBlendable _returnvalue_2 (Variables|Default|GetFadeMaterial) 1.0 :!class /Script/Engine.PostProcessVolume)
    (bind _newtrack_0 (Timeline|Timeline PlayFromStart)
      (:Update
        (Rendering|Material|SetScalarParameterValue (Variables|Default|GetFadeMaterial) "Alpha" _newtrack_0 :!class /Script/Engine.MaterialInstanceDynamic)
        (if (== _newtrack_0 1.0)
          (CallFunction|OnFixedCamOverlap))))))

(event Custom|ResetCam
  (Game|Player|SetViewTargetwithBlend (Game|GetPlayerController 0) self 1.0 (Variables|Default|GetBlend%20Func) 0.0 false))

(event Custom|Activate%20Tint
  (if (not (Variables|Default|GetGlint%20Active))
    (Variables|Default|SetGlint%20Active true)
    (bind _newtrack_0 (Timeline|Timeline_0 PlayFromStart)
      (:Update
        (Class|CameraComponent|SetPostProcessBlendWeight (Variables|Default|GetCineCamera) _newtrack_0))
      (:Finished
        (Variables|Default|SetGlint%20Active false)))))

(event EventBeginPlay
  (Utilities|FlowControl|Delay 0.2)
  (if (Variables|Default|GetIsStartingCamera)
    (CallFunction|OnFixedCamOverlap)))

(event EventTick
  (params (DeltaSeconds :type Float%20%28single-precision%29))
  (bind _returnvalue (Game|Player|GetPlayerPawn 0))
  (bind _cinecamera (Variables|Default|GetCineCamera))
  (bind _returnvalue_2 (Transformation|GetActorLocation _returnvalue))
  (bind _returnvalue_3 (Transformation|GetWorldLocation _cinecamera))
  (bind _returnvalue_4 (Math|Rotator|FindLookatRotation _returnvalue_3 _returnvalue_2))
  (Transformation|SetWorldRotation (Variables|Default|GetCineCamera) (Math|Interpolation|RInterpTo (Transformation|GetWorldRotation _cinecamera) (Math|Rotator|MakeRotator 0.0 (Math|Float|Clamp(Float) (.pitch _returnvalue_4) -65.0 0.0) (Math|Float|Clamp(Float) (.yaw _returnvalue_4) -3e+01 3e+01)) DeltaSeconds (Variables|Default|GetInterp%20Speed_0)) false false))

(fn ConstructionScript)

(fn OnFixedCamOverlap
  (Actor|Tick|SetActorTickEnabled true)
  (Game|Player|SetViewTargetwithBlend (Game|GetPlayerController 0) self (Variables|Default|GetBlend%20Time) (Variables|Default|GetBlend%20Func) 0.0 false))
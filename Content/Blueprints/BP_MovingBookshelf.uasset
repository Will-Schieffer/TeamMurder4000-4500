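; Interactive bookshelf puzzle actor that slides aside once the player finds and clicks its trigger mesh.
; Interacting blends the view to a bookshelf camera and shows the cursor; an escape event can back out.
; Clicking the placeholder mesh plays sounds, slides the shelf, destroys the interaction components, then ends BP_Player's book interaction and resets the default camera.
; A separate event briefly flashes a Niagara glint as an interaction hint.
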(event OnClicked(PlaceholderMesh)
  (params (TouchedComponent :type Primitive%20Component%20Object%20Reference) (ButtonPressed :type Key%20Structure :default "None"))
  ;[0.15 0.15 0.15 0.5] Reset back to default after puzzle solved
  (Variables|/Script/Engine.PlayerController|SetbShowMouseCursor (Game|GetPlayerController 0) false)
  (Audio|PlaySound2D "/Game/SoundFX/ButtonPush.ButtonPush" 1.0 1.0 0.0 0 0)
  (Utilities|FlowControl|Delay 0.8)
  (CallFunction|MoveBookshelfRight)
  (Audio|PlaySound2D "/Game/SoundFX/SlidingDoor.SlidingDoor" 1.0 1.0 0.0 0 0)
  (Utilities|FlowControl|Delay 2.0)
  (bind _asbp_player (Utilities|Casting|CastToBP_Player (Game|GetPlayerCharacter 0)))
  (Default|EndBookInteraction _asbp_player)
  (Default|ResetCam (Variables|Default|GetDefaultCam)))

(event Custom|EscapeInteraction
  (params (TouchedComponent :type Primitive%20Component%20Object%20Reference) (ButtonPressed :type Key%20Structure :default "None"))
  ;[0.15 0.15 0.15 0.5] Escape Bookshelf Interaction
  (if (Variables|Default|GetInteractionActive)
    (Variables|/Script/Engine.PlayerController|SetbShowMouseCursor (Game|GetPlayerController 0) false)
    (bind _asbp_player (Utilities|Casting|CastToBP_Player (Game|GetPlayerCharacter 0)))
    (Default|EndBookInteraction _asbp_player)
    (Default|ResetCam (Variables|Default|GetDefaultCam))))

(event Custom|ActivateGlint
  ;[0.15 0.15 0.15 0.5] Glint Stuff
  (Components|Activation|Activate (Variables|Default|GetNS_Interaction) false)
  (Utilities|FlowControl|Delay 5.0)
  (Components|Activation|Deactivate (Variables|Default|GetNS_Interaction)))

(event Custom|Move%20Bookshelf%20Right
  (bind _bookshelfmulticolor (Variables|Default|GetBookshelfMulticolor))
  ;[0.15 0.15 0.15 0.5] Move Bookshelf Event
  (Components|MoveComponentTo _bookshelfmulticolor (+ (Variables|/Script/Engine.SceneComponent|GetRelativeLocation _bookshelfmulticolor) "100.000000,0.000000,0.000000") "0, 0, 0" false false 2.0 false)
  (Components|DestroyComponent (Variables|Default|GetBox))
  (Variables|Default|SetCanInteract false)
  (Components|DestroyComponent (Variables|Default|GetPlaceholderMesh))
  (Components|DestroyComponent (Variables|Default|GetBookshelfGlow)))

(event Custom|BookshelfInteractedWIth
  ;[0.15 0.15 0.15 0.5] Interaction
  (Game|Player|SetViewTargetwithBlend (Game|GetPlayerController 0) (Variables|Default|GetBookShelfCam) 0.5 "VTBlend_Linear" 0.0 false)
  (Utilities|FlowControl|Delay 0.5)
  (Variables|/Script/Engine.PlayerController|SetbShowMouseCursor (Game|GetPlayerController 0) true)
  (Variables|Default|SetInteractionActive true))

(fn ConstructionScript)
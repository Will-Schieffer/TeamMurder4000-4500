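; Suitcase puzzle actor that opens on a combination check, revealing a stored souvenir and note.
; The check chains equality tests on three slot booleans rather than ANDing them, so it passes when any odd number are true.
; Success plays a sound, destroys the box component, closes the menu, restores game input and marks the puzzle done.
; A separate event briefly activates a Niagara interaction glint.
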(event Custom|CheckCombination
  (params (menu :type Suitcase%20Menu%20Object%20Reference))
  (if (== (== (== (Variables|Default|Getslot1) true) (== (Variables|Default|Getslot2) true)) (== (Variables|Default|Getslot3) true))
    (Audio|PlaySound2D "/Game/SoundFX/ItemPickUpPop1.ItemPickUpPop1" 1.0 1.0 0.0 0 0)
    (Components|DestroyComponent (Variables|Default|GetBox))
    (Widget|RemovefromParent menu)
    (Input|SetInputModeGameOnly (Game|GetPlayerController 0) false)
    (Variables|/Script/Engine.PlayerController|SetbShowMouseCursor (Game|GetPlayerController 0) false)
    (Rendering|SetActorHiddenInGame (Variables|Default|GetStoredSouvenir) false)
    (Rendering|SetActorHiddenInGame (Variables|Default|GetStoredNote) false)
    (Variables|Default|SetpuzzleDone true)))

(event Custom|ActivateGlint
  (Components|Activation|Activate (Variables|Default|GetNS_Interaction) false)
  (Utilities|FlowControl|Delay 5.0)
  (Components|Activation|Deactivate (Variables|Default|GetNS_Interaction)))

(event EventBeginPlay
  (Variables|Default|SetpuzzleDone false))

(fn ConstructionScript)
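; BP_Souvenir is a collectable souvenir that the player picks up and adds to their CollectedSouvenirs list.
; allowcollect blocks pickup of a Stored souvenir until the Suitcase puzzle is done, while unstored ones collect immediately.
; Collection notifies BP_PuzzleGate, plays a pickup sound and teleports the actor far away instead of destroying it.
; ActivateGlint briefly runs the NSCollectable effect, then switches it off after a delay.
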(event Custom|AddToInventory
  (params (Player :type BP%20Player%20Object%20Reference))
  (Utilities|Array|Add (Variables|/Game/Blueprints/BP_Player.BP_Player_C|GetCollectedSouvenirs Player) self))

(event Custom|ActivateGlint
  (Components|Activation|Activate (Variables|Default|GetNS_Collectable) false)
  (Utilities|FlowControl|Delay 5.0)
  (Components|Activation|Deactivate (Variables|Default|GetNS_Collectable)))

(event Custom|allowcollect
  (params (Player :type BP%20Player%20Object%20Reference))
  (if (Variables|Default|Getstored)
    (bind _returnvalue (Actor|GetActorOfClass "/Game/Blueprints/suitcase.suitcase_C"))
    (if (Variables|/Game/Blueprints/suitcase.suitcase_C|GetpuzzleDone _returnvalue)
      (bind _returnvalue_2 (Actor|GetActorOfClass "/Game/Blueprints/BP_PuzzleGate.BP_PuzzleGate_C" :!label _label))
      (Default|CollectItem _returnvalue_2)
      (Audio|PlaySound2D "/Game/SoundFX/ItemPickup1.ItemPickup1" 1.0 1.0 0.0 0 0)
      (CallFunction|AddtoInventory Player)
      (Transformation|Teleport "-1000.000000,-1000.000000,-1000.000000" "0, 0, 0"))
    (else
      (goto _label))))

(fn ConstructionScript)
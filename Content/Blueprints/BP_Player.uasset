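; Player Blueprint for an exploration puzzle game, handling interaction and item highlighting, and starting eerie background music on BeginPlay.
; E acts on overlapping portraits, notes, souvenirs, bookshelves and puzzle gates, with separate handlers per type.
; Gates open a UI-only souvenir-check widget, while bookshelves hide the player until EndBookInteraction and receive both interact and escape calls.
; Q triggers a glint on every souvenir, bookshelf and note in the level.
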(event Custom|EndBookInteraction
  ;[0.15 0.15 0.15 0.5] Bookshelf interaction stuff
  (Rendering|SetActorHiddenInGame false))

(event EventBeginPlay
  (Audio|PlaySound2D "/Game/SoundFX/EerieBackgroundMusic.EerieBackgroundMusic" 1.0 1.0 0.0 0 0))

(event Input|KeyboardEvents|Q
  (params (Key :type Key%20Structure :default "None"))
  (:Pressed
    (bind _outactors (Actor|GetAllActorsOfClass "/Game/Notes/BP_Note1.BP_Note1_C"))
    (for _array_element _outactors
      (Default|ActivateGlint _array_element))))

(event Input|KeyboardEvents|E
  (params (Key :type Key%20Structure :default "None"))
  (bind _returnvalue (Game|GetPlayerController 0))
  (:Pressed
    (for _array_element (Collision|GetOverlappingActors "/Game/Blueprints/BP_PuzzleGate.BP_PuzzleGate_C" :!class /Script/Engine.Actor)
      (bind _returnvalue_2 (UserInterface|CreateWidget "/Game/DragAndDrop/WB_Background.WB_Background_C"))
      (UserInterface|Viewport|AddtoViewport _returnvalue_2 0)
      (Variables|/Script/Engine.PlayerController|SetbShowMouseCursor _returnvalue true)
      (Input|SetInputModeUIOnly _returnvalue 0 "DoNotLock" false)
      (Default|CheckSouvenirs _returnvalue_2 self)
      (Utilities|Casting|CastToBP_PuzzleGate _array_element))))

(event Input|KeyboardEvents|E
  (params (Key :type Key%20Structure :default "None"))
  ;[0.15 0.15 0.15 0.5] Escape Bookshelf Interaction
  (:Pressed
    (for _array_element (Collision|GetOverlappingActors "/Game/Blueprints/BP_MovingBookshelf.BP_MovingBookshelf_C" :!class /Script/Engine.Actor)
      (bind _asbp_moving_bookshelf (Utilities|Casting|CastToBP_MovingBookshelf _array_element))
      (Rendering|SetActorHiddenInGame true)
      (Default|EscapeInteraction _asbp_moving_bookshelf 0 "None"))))

(event Input|KeyboardEvents|E
  (params (Key :type Key%20Structure :default "None"))
  (:Pressed
    (for _array_element (Collision|GetOverlappingActors "/Game/Portrait/BP_Portrait.BP_Portrait_C" :!class /Script/Engine.Actor)
      (bind _asbp_portrait (Utilities|Casting|CastToBP_Portrait _array_element))
      (Default|PortraitCloseup _asbp_portrait))))

(event Input|KeyboardEvents|E
  (params (Key :type Key%20Structure :default "None"))
  (:Pressed
    (for _array_element (Collision|GetOverlappingActors "/Game/Blueprints/BP_Souvenir.BP_Souvenir_C" :!class /Script/Engine.Actor)
      (bind _asbp_souvenir (Utilities|Casting|CastToBP_Souvenir _array_element))
      (Default|Allowcollect _asbp_souvenir self))))

(event Input|KeyboardEvents|E
  (params (Key :type Key%20Structure :default "None"))
  ;[0.15 0.15 0.15 0.5] Bookshelf interaction stuff
  (:Pressed
    (for _array_element (Collision|GetOverlappingActors "/Game/Blueprints/BP_MovingBookshelf.BP_MovingBookshelf_C" :!class /Script/Engine.Actor)
      (bind _asbp_moving_bookshelf (Utilities|Casting|CastToBP_MovingBookshelf _array_element))
      (Rendering|SetActorHiddenInGame true)
      (Default|BookshelfInteractedWIth _asbp_moving_bookshelf))))

(event Input|KeyboardEvents|Q
  (params (Key :type Key%20Structure :default "None"))
  (:Pressed
    (bind _outactors (Actor|GetAllActorsOfClass "/Game/Blueprints/BP_Souvenir.BP_Souvenir_C"))
    (for _array_element _outactors
      (Default|ActivateGlint _array_element))))

(event Input|KeyboardEvents|Q
  (params (Key :type Key%20Structure :default "None"))
  (:Pressed
    (bind _outactors (Actor|GetAllActorsOfClass "/Game/Blueprints/BP_MovingBookshelf.BP_MovingBookshelf_C"))
    (for _array_element _outactors
      (Default|ActivateGlint _array_element))))

(event Input|KeyboardEvents|E
  (params (Key :type Key%20Structure :default "None"))
  (:Pressed
    (for _array_element (Collision|GetOverlappingActors "/Game/Notes/BP_Note1.BP_Note1_C" :!class /Script/Engine.Actor)
      (bind _asbp_note_1 (Utilities|Casting|CastToBP_Note1 _array_element))
      (Default|ShowNote _asbp_note_1))))

(fn ConstructionScript)
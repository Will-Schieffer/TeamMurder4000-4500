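; BP_Dave is a talkable Blueprint, apparently an NPC, that shows dialogue one line at a time.
; Each Talk event increments TextInd and writes that DialogueText entry into a BW_Dialogue widget, created and added to the viewport when no valid one exists.
; Once the index passes the last line, the widget is removed from its parent; the index is not reset here.
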(event EventTalk
  (bind _text_ind (Variables|Default|GetText_Ind))
  (Math|Integer|IncrementInt _text_ind
    (:%20%20
      (if (< _text_ind (Utilities|Array|Length (Variables|Default|GetDialogue_Text)))
        (Variables|Default|GetText_UI
          (:then
            _)
          (:else
            (bind _returnvalue (UserInterface|CreateWidget "/Game/UI/BW_Dialogue.BW_Dialogue_C" (Game|GetPlayerController 0)))
            (bind _output_get (Variables|Default|SetText_UI _returnvalue))
            (UserInterface|Viewport|AddtoViewport _output_get 0)))
        (Rendering|Components|TextRender|SetText (Variables|/Game/UI/BW_Dialogue.BW_Dialogue_C|GetWB_Dialogue (Variables|Default|GetText_UI)) (Utilities|Text|ToText(String) (Utilities|Array|Get(acopy) (Variables|Default|GetDialogue_Text) (Variables|Default|GetText_Ind))))
        (else
          (Widget|RemovefromParent (Variables|Default|GetText_UI)))))))

(fn ConstructionScript)
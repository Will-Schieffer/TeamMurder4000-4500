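; BP_Portrait is a portrait actor that toggles a close-up view for the player.
; Its PortraitCloseup event uses a FlipFlop to alternate between entering and leaving the close-up.
; Entering blends the first player controller's view target to the portrait and ignores look and move input.
; Leaving calls ResetCam on DefaultCam and stops ignoring that input.
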(event Custom|PortraitCloseup
  (bind _returnvalue (Game|GetPlayerController 0))
  (bind _returnvalue_2 (Game|GetPlayerController 0))
  (Utilities|FlowControl|FlipFlop
    (:A
      (Game|Player|SetViewTargetwithBlend _returnvalue_2 self 0.5 "VTBlend_Linear" 0.0 false)
      (Input|SetIgnoreLookInput _returnvalue_2 true)
      (Input|SetIgnoreMoveInput _returnvalue_2 true))
    (:B
      (Default|ResetCam (Variables|Default|GetDefaultCam))
      (Input|SetIgnoreLookInput _returnvalue false)
      (Input|SetIgnoreMoveInput _returnvalue false))))

(fn ConstructionScript)